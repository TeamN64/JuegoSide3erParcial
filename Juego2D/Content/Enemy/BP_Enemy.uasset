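; Enemy pawn that wanders, can chase the player, and is destroyed by a BP_ProjectileB hit with a sound and Niagara effect.
; Wandering picks a nearby random reachable point every second until pawn sensing spots the player, which sets IsSeen and triggers a jump.
; RangeCheck, which nothing here calls, either resumes wandering when the player is far or starts an AIMoveTo chase that retries on failure.
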(event OnSeePawn(PawnSensing)
  (params (Pawn :type Pawn%20Object%20Reference))
  (Utilities|Casting|CastToBP_Player Pawn)
  (Character|Jump)
  (Variables|Default|SetIsSeen true)
  (CallFunction|WonderAurond))

(event OnComponentHit(CapsuleComponent)
  (params (HitComponent :type Primitive%20Component%20Object%20Reference) (OtherActor :type Actor%20Object%20Reference) (OtherComp :type Primitive%20Component%20Object%20Reference) (NormalImpulse :type Vector :default "0, 0, 0") (Hit :type Hit%20Result%20Structure%20%28by%20ref%29))
  (bind _returnvalue (Transformation|GetActorLocation))
  (Utilities|Casting|CastToBP_ProjectileB OtherActor)
  (Audio|PlaySoundatLocation 0 _returnvalue "0, 0, 0" 1.0 1.0 0.0 0 0 0 0)
  (Niagara|SpawnSystematLocation "/Game/NS/NS_CoinPickup.NS_CoinPickup" _returnvalue "0, 0, 0" "1.000000,1.000000,1.000000" true true "AutoRelease")
  (Actor|DestroyActor))

(event Custom|ChasePlayer
  (bind _returnvalue (Game|GetPlayerCharacter 0))
  (if (and (Variables|Default|GetIsSeen) (not (AI|Components|NavMovement|IsFalling (Variables|Character|GetCharacterMovement)))) :!label _label
    (AI|AIMoveTo self (Transformation|GetActorLocation _returnvalue) _returnvalue 2e+01 false
      (:OnFail
        (Utilities|FlowControl|Delay 0.2)
        (goto _label)))
    (else
      (CallFunction|WonderAurond))))

(event Custom|WonderAurond
  (bind _self self)
  (if (not (Variables|Default|GetIsSeen)) :!label _label
    (AI|Navigation|SimpleMovetoLocation (Pawn|GetController _self) (.RandomLocation (AI|Navigation|GetRandomReachablePointinRadius (Transformation|GetActorLocation _self) 3e+02 0 0)))
    (Utilities|FlowControl|Delay 1.0)
    (goto _label)))

(event Custom|RangeCheck
  (if (> (Transformation|GetDistanceTo self (Game|GetPlayerCharacter 0)) 2.5e+02)
    (Variables|Default|SetIsSeen false)
    (CallFunction|WonderAurond)
    (else
      (CallFunction|ChasePlayer))))

(event EventBeginPlay
  (CallFunction|WonderAurond))

(fn ConstructionScript)