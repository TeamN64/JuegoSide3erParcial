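; BP_Palanca is a lever target that is destroyed when a BP_ProjectileB overlaps its Box component.
; On that hit it also decrements the Amount counter in BP_GameMode1 by one.
; BeginPlay writes the same counter back minus zero, leaving it unchanged, and a leftover debug print is never executed.
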(event OnComponentBeginOverlap(Box)
  (params (OverlappedComponent :type Primitive%20Component%20Object%20Reference) (OtherActor :type Actor%20Object%20Reference) (OtherComp :type Primitive%20Component%20Object%20Reference) (OtherBodyIndex :type Integer) (bFromSweep :type Boolean) (SweepResult :type Hit%20Result%20Structure%20%28by%20ref%29))
  (Utilities|Casting|CastToBP_ProjectileB OtherActor)
  (Actor|DestroyActor)
  (bind _asbp_game_mode_1 (Utilities|Casting|CastToBP_GameMode1 (Game|GetGameMode)))
  (Variables|/Game/GameMode/BP_GameMode1.BP_GameMode1_C|SetAmount _asbp_game_mode_1 (- (Variables|/Game/GameMode/BP_GameMode1.BP_GameMode1_C|GetAmount _asbp_game_mode_1) 1)))

(event EventBeginPlay
  (bind _asbp_game_mode_1 (Utilities|Casting|CastToBP_GameMode1 (Game|GetGameMode)))
  (Variables|/Game/GameMode/BP_GameMode1.BP_GameMode1_C|SetAmount _asbp_game_mode_1 (- (Variables|/Game/GameMode/BP_GameMode1.BP_GameMode1_C|GetAmount _asbp_game_mode_1) 0)))

(event Collision|EventActorBeginOverlap
  (params (OtherActor :type Actor%20Object%20Reference)))

(event EventTick
  (params (DeltaSeconds :type Float%20%28single-precision%29)))

(fn ConstructionScript)