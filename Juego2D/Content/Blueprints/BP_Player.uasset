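; BP_Player is the player character, which moves on one input axis, jumps, stomps enemies and spawns projectiles.
; BeginPlay creates the HUD and health bar widgets and adds the Enhanced Input mapping context.
; Landing on a BP_Enemy destroys it and launches the player upward by BounceHeight.
; Pressing J spawns an actor at SpawnBullet, while the timer-based auto-fire is unwired and its event is empty.
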(event Custom|spawnProyectil)

(event Input|EnhancedActionEvents|EnhancedInputActionMovement
  (params (ActionValue :type Float%20%28double-precision%29) (ElapsedSeconds :type Float%20%28double-precision%29) (TriggeredSeconds :type Float%20%28double-precision%29) (InputAction :type Input%20Action%20Object%20Reference :default "/Game/Inputs/Movement.Movement"))
  (:Triggered
    (Pawn|Input|AddMovementInput (Math|Vector|GetForwardVector (Math|Rotator|MakeRotator 0.0 0.0 (.yaw (Pawn|GetControlRotation :!class /Script/Engine.Pawn)))) ActionValue false)))

(event Input|EnhancedActionEvents|EnhancedInputActionJump
  (params (ActionValue :type Boolean) (ElapsedSeconds :type Float%20%28double-precision%29) (TriggeredSeconds :type Float%20%28double-precision%29) (InputAction :type Input%20Action%20Object%20Reference :default "/Game/Inputs/Jump.Jump"))
  (:Triggered
    (Character|Jump))
  (:Completed
    (Character|StopJumping)))

(event EventOnLanded
  (params (Hit :type Hit%20Result%20Structure%20%28by%20ref%29))
  (bind _asbp_enemy (Utilities|Casting|CastToBP_Enemy (.HitActor (Collision|BreakHitResult Hit))))
  (Actor|DestroyActor _asbp_enemy)
  (Character|LaunchCharacter (* (Math|Vector|VectorUp) (Variables|Default|GetBounceHeight)) false false))

(event EventBeginPlay
  (Utilities|FlowControl|Sequence
    (:then_0
      (bind _returnvalue (UserInterface|CreateWidget "/Game/Widgets/W_HUD.W_HUD_C"))
      (UserInterface|Viewport|AddtoViewport _returnvalue 0)
      (bind _asplayer_controller (Utilities|Casting|CastToPlayerController (Pawn|GetController)))
      (Utilities|IsValid (PlayerController|LocalPlayerSubsystems|GetEnhancedInputLocalPlayerSubsystem _asplayer_controller)
        (:Is%20Valid
          (Input|AddMappingContext (PlayerController|LocalPlayerSubsystems|GetEnhancedInputLocalPlayerSubsystem _asplayer_controller) "/Game/Inputs/IMC_Default.IMC_Default" 0 "(bIgnoreAllPressedKeysUntilRelease=True,bForceImmediately=False)"))))
    (:then_1
      ;[1 1 1] Show Health Bar in the Screen
      (bind _returnvalue_2 (UserInterface|CreateWidget "/Game/Widgets/WPB_HealthBar.WPB_HealthBar_C"))
      (UserInterface|Viewport|AddtoViewport _returnvalue_2 0))))

(event Input|KeyboardEvents|J
  (params (Key :type Key%20Structure :default "None"))
  (:Pressed
    (Game|SpawnActorfromClass "/Game/Blueprints/BP_ProjectileB.BP_ProjectileB_C" (Transformation|GetWorldTransform (Variables|Default|GetSpawnBullet)) "AlwaysSpawn" "MultiplyWithRoot" 0 0)))

(fn ConstructionScript)