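; Actor component that tracks health for its owning actor and reports changes through event dispatchers.
; On BeginPlay it fills health to max and binds to the owner's OnTakeAnyDamage.
; Each hit subtracts damage, clamps between zero and max, broadcasts OnHealthChanged, and fires OnHealthDepleted whenever health is at zero, with no guard against repeat calls.
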(event Custom|OnDamageTaken
  (params (DamagedActor :type Actor%20Object%20Reference) (Damage :type Float%20%28single-precision%29) (DamageType :type Damage%20Type%20Object%20Reference) (InstigatedBy :type Controller%20Object%20Reference) (DamageCauser :type Actor%20Object%20Reference))
  (bind _output_get (Variables|Default|SetHealth (Math|Float|Clamp(Float) (- (Variables|Default|GetHealth) Damage) 0.0 (Variables|Default|GetMaxHealth))))
  (Default|CallOnHealthChanged _output_get (Variables|Default|GetMaxHealth))
  (if (<= (Variables|Default|GetHealth) 0.0)
    (Default|CallOnHealthDepleted)))

(event EventBeginPlay
  (Variables|Default|SetHealth (Variables|Default|GetMaxHealth))
  (EventDispatchers|BindEventtoOnTakeAnyDamage (Components|GetOwner) (delegate Custom|OnDamageTaken)))