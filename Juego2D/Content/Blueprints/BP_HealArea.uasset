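; BP_HealArea is an area actor that periodically heals players standing inside it.
; HealCollision overlap events add and remove BP_Player actors in the ActorsHeal array.
; A looping timer started on BeginPlay fires HealTick every half second, which checks each tracked player's BPHealthComponent.
; Players below max health are healed through ApplyDamage with a negated HealingAmount, reusing the damage path instead of a separate heal call.
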(event OnComponentBeginOverlap(HealCollision)
  (params (OverlappedComponent :type Primitive%20Component%20Object%20Reference) (OtherActor :type Actor%20Object%20Reference) (OtherComp :type Primitive%20Component%20Object%20Reference) (OtherBodyIndex :type Integer) (bFromSweep :type Boolean) (SweepResult :type Hit%20Result%20Structure%20%28by%20ref%29))
  (bind _asbp_player (Utilities|Casting|CastToBP_Player OtherActor))
  (Utilities|IsValid _asbp_player
    (:Is%20Valid
      (Utilities|Array|Add (Variables|Default|GetActor'sHeal) _asbp_player))))

(event OnComponentEndOverlap(HealCollision)
  (params (OverlappedComponent :type Primitive%20Component%20Object%20Reference) (OtherActor :type Actor%20Object%20Reference) (OtherComp :type Primitive%20Component%20Object%20Reference) (OtherBodyIndex :type Integer))
  (bind _asbp_player (Utilities|Casting|CastToBP_Player OtherActor))
  (if (>= (Utilities|Array|FindItem (Variables|Default|GetActor'sHeal) _asbp_player) 0)
    (Utilities|Array|RemoveIndex (Variables|Default|GetActor'sHeal) (Utilities|Array|FindItem (Variables|Default|GetActor'sHeal) _asbp_player))))

(event Custom|HealTick
  (for _array_element (Variables|Default|GetActor'sHeal)
    (bind _asbp_player (Utilities|Casting|CastToBP_Player _array_element))
    (if (< (Variables|/Game/Blueprints/BP_HealthComponent.BP_HealthComponent_C|GetHealth (Variables|/Game/Blueprints/BP_Player.BP_Player_C|GetBP_HealthComponent _asbp_player)) (Variables|/Game/Blueprints/BP_HealthComponent.BP_HealthComponent_C|GetMaxHealth (Variables|/Game/Blueprints/BP_Player.BP_Player_C|GetBP_HealthComponent _asbp_player)))
      (Game|Damage|ApplyDamage _array_element (* (Variables|Default|GetHealingAmount) -1.0) 0 0))))

(event EventBeginPlay
  (Utilities|Time|SetTimerbyEvent (delegate Custom|HealTick) 0.5 true))

(fn ConstructionScript)