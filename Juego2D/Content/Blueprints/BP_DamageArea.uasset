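; BP_DamageArea is a single-use damage volume that applies BaseDamage to overlapping actors that have a BP_HealthComponent.
; DamageCollision begin and end overlap events keep the ActorsToDamage list current.
; A fast looping timer started on BeginPlay damages every listed actor.
; DestroyActor is called inside that loop, so the area removes itself on the first tick that finds a target.
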(event OnComponentBeginOverlap(DamageCollision)
  (params (OverlappedComponent :type Primitive%20Component%20Object%20Reference) (OtherActor :type Actor%20Object%20Reference) (OtherComp :type Primitive%20Component%20Object%20Reference) (OtherBodyIndex :type Integer) (bFromSweep :type Boolean) (SweepResult :type Hit%20Result%20Structure%20%28by%20ref%29))
  (Utilities|IsValid (Actor|GetComponentbyClass OtherActor "/Game/Blueprints/BP_HealthComponent.BP_HealthComponent_C")
    (:Is%20Valid
      (Utilities|Array|Add (Variables|Default|GetActor'sToDamage) OtherActor))))

(event OnComponentEndOverlap(DamageCollision)
  (params (OverlappedComponent :type Primitive%20Component%20Object%20Reference) (OtherActor :type Actor%20Object%20Reference) (OtherComp :type Primitive%20Component%20Object%20Reference) (OtherBodyIndex :type Integer))
  (bind _actor_stodamage (Variables|Default|GetActor'sToDamage))
  (bind _returnvalue (Utilities|Array|FindItem _actor_stodamage OtherActor))
  (if (>= _returnvalue 0)
    (Utilities|Array|RemoveIndex (Variables|Default|GetActor'sToDamage) _returnvalue)))

(event Custom|DamageTick
  (for _array_element (Variables|Default|GetActor'sToDamage)
    (Game|Damage|ApplyDamage _array_element (Variables|Default|GetBaseDamage) 0 0)
    (Actor|DestroyActor)))

(event EventBeginPlay
  (Utilities|Time|SetTimerbyEvent (delegate Custom|DamageTick) 0.1 true))

(fn ConstructionScript)